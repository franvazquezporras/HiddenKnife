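; BP_AI_Boss is a boss AI Blueprint that reports its health to its AI controller.
; Every Tick, after the parent Tick, it casts its controller to BP_AIController_Boss and copies CurrentHealth and MaxHealth from BPCPlayerStats into that controller.
; The update is polled each frame, and the Blueprint adds no other logic of its own beyond parent calls.
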(event EventBeginPlay
  (|CallParentFunction) ; This node is disabled and will not be called.\nDrag off pins to build functionality.
)

(event Collision|EventActorBeginOverlap
  (params (OtherActor :type Actor%20Object%20Reference))
  (|CallParentFunction OtherActor) ; This node is disabled and will not be called.\nDrag off pins to build functionality.
)

(event EventTick
  (params (DeltaSeconds :type Float%20%28single-precision%29))
  (bind _bpc_playerstats (Variables|Default|GetBPC_PlayerStats))
  (|CallParentFunction DeltaSeconds)
  (bind _asbp_aicontroller_boss (Utilities|Casting|CastToBP_AIController_Boss (AI|GetAIController self)))
  (Variables|/Game/AI/Boss/BP_AIController_Boss.BP_AIController_Boss_C|Sethealth _asbp_aicontroller_boss (Variables|/Game/Blueprints/BPC_PlayerStats.BPC_PlayerStats_C|GetCurrent%20Health _bpc_playerstats))
  (Variables|/Game/AI/Boss/BP_AIController_Boss.BP_AIController_Boss_C|SetmaxHealth _asbp_aicontroller_boss (Variables|/Game/Blueprints/BPC_PlayerStats.BPC_PlayerStats_C|GetMax%20Health _bpc_playerstats)))

(fn ConstructionScript
  (|CallParentFunction))