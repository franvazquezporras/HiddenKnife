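; Equipment component for the third-person character that lets the player pick up weapons and keeps a list of them.
; On interact, it sphere-traces forward from the owner's follow camera and, on hitting a BP_Weapon, stores that weapon's item data and destroys the actor.
; Collected items accumulate in the WeaponSlots array with no capacity or duplicate check.
; A debug key prints each stored item's row name.
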(event Input|EnhancedActionEvents|EnhancedInputActionIA_Interact
  (params (ActionValue :type Boolean) (ElapsedSeconds :type Float%20%28double-precision%29) (TriggeredSeconds :type Float%20%28double-precision%29) (InputAction :type Input%20Action%20Object%20Reference :default "/Game/ThirdPerson/Input/Actions/IA_Interact.IA_Interact"))
  (bind _follow_camera (Variables|Default|GetFollow%20Camera))
  (bind _returnvalue (Transformation|GetWorldLocation _follow_camera))
  ;[0.05127 0.05127 0.05127] Pick Up trace
  (:Started
    (bind (_outhit _returnvalue_2) (Collision|SphereTraceForObjects _returnvalue (+ _returnvalue (* (Math|Vector|GetForwardVector (Transformation|GetWorldRotation _follow_camera)) 1e+03)) 15.0 (Utilities|Array|MakeArray "ObjectTypeQuery2") false 0 "ForDuration"))
    (if _returnvalue_2
      (bind _asbp_weapon (Utilities|Casting|CastToBP_Weapon (.HitActor (Collision|BreakHitResult _outhit))))
      (CallFunction|AddWeapon (Variables|/Game/Equipment_System/BP_Weapon.BP_Weapon_C|GetItemData _asbp_weapon))
      (Actor|DestroyActor _asbp_weapon)
      (Development|PrintString "Item Gathered"))))

(event EventBeginPlay
  (bind _asbp_third_person_character (Utilities|Casting|CastToBP_ThirdPersonCharacter (Components|GetOwner)))
  (Variables|Default|SetFollow%20Camera (Variables|/Game/ThirdPerson/Blueprints/BP_ThirdPersonCharacter.BP_ThirdPersonCharacter_C|GetFollowCamera _asbp_third_person_character)))

(event Input|KeyboardEvents|DebugKeyH
  (params (Key :type Key%20Structure :default "None") (ActionValue :type Input%20Action%20Value%20Structure))
  ;[0.05127 0.05127 0.05127] Pick Up trace
  (:Pressed
    (for _array_element (Variables|Default|GetweaponSlots)
      (Development|PrintString (Utilities|String|ToString(Name) (.rowname (.item _array_element))) true true "(R=0.000000,G=0.660000,B=1.000000,A=1.000000)" 5.0))))

(fn AddWeapon
  (params (NewItem :type S%20Slots%20Structure%20%28by%20ref%29))
  (Utilities|Array|Add (Variables|Default|GetweaponSlots) NewItem))